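; Game instance that handles pausing, level travel, global audio options and save clearing.
; Pause toggles WB_PauseMenu and the cursor, with unpausing deferring to the player controller's Inventory state to decide whether the game stays paused.
; Loading or restarting the game level shows a loading screen that plays until stopped.
; Options persist in a "GlobalOptions" save slot, created if missing, and drive music and SFX volume through sound mix overrides.
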(event `pauseGame`
  (if (`self.bPauseMenu`)
    (`GameplayStatics.SetGamePaused` (`/Game/BluePrints/BP_ExamPlayerController.bInventory` (`/Game/BluePrints/BP_ExamFunctionLibrary.GetPlayerControllerBP`)))
    (`/Game/BluePrints/WidgetBP/WB_PauseMenu.CloseOptionsScreen` (stale _returnvalue))
    (set `self.bPauseMenu` false)
    (else
      (bind _returnvalue (`|CreateWidget` "/Game/BluePrints/WidgetBP/WB_PauseMenu.WB_PauseMenu_C" (`GameplayStatics.GetPlayerController` 0)))
      (`UserWidget.AddToViewport` _returnvalue 0)
      (`GameplayStatics.SetGamePaused` true)
      (set `self.bPauseMenu` true)))
  (`/Game/BluePrints/BP_ExamFunctionLibrary.ShowMouseCursor` (`self.bPauseMenu`)))

(event `GoToMainMenu`
  (`GameplayStatics.OpenLevel` "ActionRPG_Main"))

(event `LoadGameLevel`
  (`WidgetLayoutLibrary.RemoveAllWidgets`)
  (`self.FadeInAndShowLoadingScreen`)
  (`GameplayStatics.OpenLevel` "ThirdPersonExampleMap"))

(event `RestartGameLevel`
  (`self.FadeInAndShowLoadingScreen`)
  (`self.LoadGameLevel`))

(fn `ClearSaveData`
  (`self.ResetSaveGame`)
  (`self.WriteSaveGame`)
  (`KismetSystemLibrary.PrintString` "Cleared Save Data"))

(fn `FadeInAndShowLoadingScreen`
  (`ExamBPFunctionLibrary.PlayLoadingScreen` true))

(fn `FadeOutAndHideLoadingScreen`
  (`ExamBPFunctionLibrary.StopLoadingScreen`))

(fn `GetGlobalOptions`
  (returns (GlobalOptions :type "/Game/BluePrints/SaveGame/GlobalOptionsStruct Structure"))
  (bind _returnvalue (`GameplayStatics.DoesSaveGameExist` "GlobalOptions"))
  (if _returnvalue
    (bind _returnvalue_2 (`GameplayStatics.LoadGameFromSlot` "GlobalOptions"))
    (bind _asglobal_options_save_game (cast `/Game/BluePrints/SaveGame/GlobalOptionsSaveGame` _returnvalue_2))
    (return (`/Game/BluePrints/SaveGame/GlobalOptionsSaveGame.GlobalOptions` _asglobal_options_save_game))
    (else
      (bind _returnvalue_3 (`GameplayStatics.CreateSaveGameObject` "/Game/BluePrints/SaveGame/GlobalOptionsSaveGame.GlobalOptionsSaveGame_C"))
      (`GameplayStatics.SaveGameToSlot` _returnvalue_3 "GlobalOptions")
      (return (`/Game/BluePrints/SaveGame/GlobalOptionsSaveGame.GlobalOptions` _returnvalue_3)))))

(fn `SetGlobalOptions`
  (params (NewOptions :type "/Game/BluePrints/SaveGame/GlobalOptionsStruct Structure") (bInstant :type Boolean))
  (locals (NewGlobalOptions :type "/Game/BluePrints/SaveGame/GlobalOptionsStruct Structure" :default (struct :`bMusic` true :`bSoundFX` true :`bVibration` true :`bCameraShake` true)))
  (bind _returnvalue (select `bool` bInstant :`false` 1.0 :!type "Float (single-precision)"))
  (bind _output_get (set `local.NewGlobalOptions` NewOptions))
  (`GameplayStatics.SetSoundMixClassOverride` "/Game/Sound/AudioClasses/SM_Mixer.SM_Mixer" "/Game/Sound/AudioClasses/SC_Music.SC_Music" (select `bool` (break `/Game/BluePrints/SaveGame/GlobalOptionsStruct` _output_get) :`false` 0.001 :`true` 1.0 :!type "Float (single-precision)") 1.0 _returnvalue)
  (`GameplayStatics.SetSoundMixClassOverride` "/Game/Sound/AudioClasses/SM_Mixer.SM_Mixer" "/Game/Sound/AudioClasses/SC_SFX.SC_SFX" (select `bool` (`.bSoundFX_3_E497AD3440E454B52500EEB9E20F72A0` (break `/Game/BluePrints/SaveGame/GlobalOptionsStruct` _output_get)) :`true` 1.0 :!type "Float (single-precision)") 1.0 _returnvalue)
  (bind _returnvalue_2 (`GameplayStatics.CreateSaveGameObject` "/Game/BluePrints/SaveGame/GlobalOptionsSaveGame.GlobalOptionsSaveGame_C"))
  (set `/Game/BluePrints/SaveGame/GlobalOptionsSaveGame.GlobalOptions` (`local.NewGlobalOptions`) _returnvalue_2)
  (`GameplayStatics.SaveGameToSlot` _returnvalue_2 "GlobalOptions"))