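; BP_ExamPlayerController is a player controller Blueprint that mainly provides helper functions for reaching the exam game's controller.
; GetPlayerControllerBP returns the PlayerController reference held by the game mode when valid, otherwise it casts player controller 0 to this class.
; GetGameModeBP casts the current game mode to BP_ExamGameModeBase, with no visible logic on either branch.
; The PlaySKippableCutscene event takes a sequence player but is an empty stub.
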(event `Play SKippable Cutscene`
  (params (SequencePlayer :type "MovieSceneSequencePlayer Object Reference")))

(fn `GetGameModeBP`
  (returns (MyGame :type "/Game/BluePrints/BP_ExamGameModeBase Object Reference"))
  (cast `/Game/BluePrints/BP_ExamGameModeBase` (`GameplayStatics.GetGameMode`)
    (:`then`
      _)
    (:`CastFailed`
      _))
  (return null))

(fn `GetPlayerControllerBP`
  (returns (Controller :type "/Game/BluePrints/BP_ExamPlayerController Object Reference"))
  (if (`KismetSystemLibrary.IsValid` (`/Game/BluePrints/BP_ExamGameModeBase.PlayerController` (`self.GetGameModeBP`)))
    (return (`/Game/BluePrints/BP_ExamGameModeBase.PlayerController` (`self.GetGameModeBP`)))
    (else
      (bind _asbp_exam_player_controller (cast `/Game/BluePrints/BP_ExamPlayerController` (`GameplayStatics.GetPlayerController` 0)))
      (return _asbp_exam_player_controller))))

(fn `UserConstructionScript`)