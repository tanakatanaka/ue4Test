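; Blueprint function library of typed getters for the Exam project's player controller, game mode and game instance.
; GetPlayerControllerBP prefers the controller stored on the game mode, falling back to casting player controller 0 when that is invalid.
; GetGameModeBP returns the cast game mode whether or not the cast succeeds.
; GetGameInstanceBP returns its cast result, but that cast is never executed.
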(fn GetPlayerControllerBP
  (if (Utilities|IsValid (Variables|/Game/BluePrints/BP_ExamGameModeBase.BP_ExamGameModeBase_C|GetPlayerController (CallFunction|GetGameModeBP)))
    (return (Variables|/Game/BluePrints/BP_ExamGameModeBase.BP_ExamGameModeBase_C|GetPlayerController (CallFunction|GetGameModeBP)))
    (else
      (bind _asbp_exam_player_controller (Utilities|Casting|CastToBP_ExamPlayerController (Game|GetPlayerController 0)))
      (return _asbp_exam_player_controller))))

(fn GetGameModeBP
  (bind _asbp_exam_game_mode_base (Utilities|Casting|CastToBP_ExamGameModeBase (Game|GetGameMode))
    (:then
      _)
    (:CastFailed
      _))
  (return _asbp_exam_game_mode_base))

(fn GetGameInstanceBP
  (return (stale _asbp_exam_game_instance)))