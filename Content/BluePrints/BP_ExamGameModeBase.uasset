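; Exam game mode that plays an intro cutscene if present, then runs timed enemy waves.
; StartGame restarts the player, starts a one-second countdown and begins spawning.
; Waves load from the WavesProgression table by row name, show start/end widgets, and spawn BP_EnemyCharacter groups at random NPC_SpawnBox actors.
; GaneOver and EnemyDestroyed are empty; the enemy-count decrement and wave check are unwired, so waves never advance.
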(event `PlayIntroScene`
  (bind _outactors (`GameplayStatics.GetAllActorsOfClass` "/Script/LevelSequence.LevelSequenceActor"))
  (if (`KismetArrayLibrary.Array_IsValidIndex` _outactors)
    (`/Game/BluePrints/BP_ExamPlayerController.Play SKippable Cutscene` (`/Game/BluePrints/BP_ExamFunctionLibrary.GetPlayerControllerBP`) (`LevelSequenceActor.SequencePlayer` (`|GetArrayItem` _outactors)))
    (else
      (`self.Start Game`))))

(event `StartPlayTimer`
  (`KismetSystemLibrary.K2_SetTimerDelegate` (delegate `UpdatePlayTime`) 1.0 true) ; Setup remaining play time counter
  (set `self.StartTime` (`GameplayStatics.GetTimeSeconds`)))

(event `UpdatePlayTime`
  (bind _output_get (set `self.BattleTime` (- (`self.BattleTime`) 1.0)))
  (message `/Game/BluePrints/WidgetBP/HUD/iHUD.UpdateTimer` (`/Game/BluePrints/BP_ExamPlayerController.OnScreenControls` (`/Game/BluePrints/BP_ExamFunctionLibrary.GetPlayerControllerBP`)) _output_get)
  (if (<= (`self.BattleTime`) 0.0)
    (`self.Gane Over`)))

(event `self.ReceiveBeginPlay`
  (`self.PlayIntroScene`))

(event `Gane Over`)

(event `Start Game`
  (if (not (`self.bGameProgress`))
    (set `self.bGameProgress` true)
    (`self.RestartPlayer` (`/Game/BluePrints/BP_ExamFunctionLibrary.GetPlayerControllerBP`))
    (`self.StartPlayTimer`)
    (`self.StartEnemySpawn`)))

(event `StartEnemySpawn`
  (if (`self.GetRandomSpawnPoint`)
    (`KismetSystemLibrary.Delay` 1.0)
    (`self.StartNewWave`)))

(event `SpawnEnemy`
  (params (NewParam :type "/Game/BluePrints/BP_EnemyCharacter Class Reference"))
  (bind _returnvalue (`|SpawnActorFromClass` NewParam (`.Transform` (`self.GetRandomSpawnPoint`)) "AdjustIfPossibleButAlwaysSpawn" "OverrideRootScale" null null))
  (`/Engine/EditorBlueprintResources/StandardMacros.IncrementInt` (`self.SpawnedEnemies`)
    (:`  `
      (add `self.OnDestroyed` _returnvalue (delegate `EnemyDestroyed`)))))

(event `EnemyDestroyed` :!signature `self.OnDestroyed`
  (params (DestroyedActor :type "Actor Object Reference")))

(event `StartNewWave`
  (bind _returnvalue (`|GetDataTableRow` "/Game/BluePrints/Progression/WavesProgression.WavesProgression" (`KismetStringLibrary.Conv_StringToName` (`KismetStringLibrary.Concat_StrStr` "Wave_" (`KismetStringLibrary.Conv_IntToString` (`self.CurrentWave`)))))
    (:`then`
      (bind (_spawngroup _wavetime) (break `/Game/BluePrints/Progression/WaveStruct` _returnvalue))
      (set `self.Wave` _spawngroup)
      (set `self.BattleTime` (`KismetMathLibrary.Conv_IntToDouble` _wavetime))
      (`self.SpawnNewWave`))
    (:`RowNotFound`
      (`self.OnAllWavesFinished`))))

(event `SpawnNextEnemiesGroup`
  (bind _enemies (break `/Game/BluePrints/Progression/SpawnGroupStruct` (`|GetArrayItem` (`self.Wave`))))
  (for _ _enemies
    (`self.SpawnEnemy` "/Game/BluePrints/BP_EnemyCharacter.BP_EnemyCharacter_C")
    (`KismetArrayLibrary.Array_Remove` _enemies))
  (`KismetArrayLibrary.Array_Remove` (`self.Wave`)))

(event `SpawnNewWave`
  (bind _returnvalue (`|CreateWidget` "/Game/BluePrints/WidgetBP/WB_WaveStart.WB_WaveStart_C"))
  (`UserWidget.AddToViewport` _returnvalue 0)
  (`KismetSystemLibrary.Delay` 3.0)
  (`self.SpawnNextEnemiesGroup`)
  (message `/Game/BluePrints/WidgetBP/HUD/iHUD.UpdateTimer` (`/Game/BluePrints/BP_ExamPlayerController.OnScreenControls` (`/Game/BluePrints/BP_ExamFunctionLibrary.GetPlayerControllerBP`)) (`self.BattleTime`)))

(event `CheckCurrentWave`
  (if (<= (`self.SpawnedEnemies`) 0)
    (if (`KismetArrayLibrary.Array_IsValidIndex` (`self.Wave`))
      (`self.SpawnNextEnemiesGroup`)
      (else
        (`KismetSystemLibrary.RetriggerableDelay` 2.0)
        (`self.OnWaveFinished`)
        (`/Engine/EditorBlueprintResources/StandardMacros.IncrementInt` (`self.CurrentWave`))))))

(event `OnAllWavesFinished`
  (`KismetSystemLibrary.PrintString` "GAME COMPLETED")
  (`self.Gane Over`))

(event `OnWaveFinished`
  (bind _returnvalue (`|CreateWidget` "/Game/BluePrints/WidgetBP/WB_WaveEnd.WB_WaveEnd_C"))
  (`UserWidget.AddToViewport` _returnvalue 0)
  (`KismetSystemLibrary.Delay` 0.2)
  (`self.StartNewWave`))

(fn `GetRandomSpawnPoint`
  (returns (Valid :type Boolean) (Transform :type "Transform Structure"))
  (locals (SpawnPoint :type "Transform Structure"))
  (bind _outactors (`GameplayStatics.GetAllActorsOfClass` "/Game/BluePrints/NPC/NPC_SpawnBox.NPC_SpawnBox_C"))
  (bind _returnvalue (`KismetArrayLibrary.Array_IsValidIndex` _outactors))
  (if _returnvalue
    (bind _output_get (set `local.SpawnPoint` (`self.GetTransform` (`|GetArrayItem` _outactors (`KismetMathLibrary.RandomInteger` (`KismetArrayLibrary.Array_LastIndex` _outactors))))))
    (return true _output_get)
    (else
      (return _returnvalue (`local.SpawnPoint`)))))

(fn `UserConstructionScript`)